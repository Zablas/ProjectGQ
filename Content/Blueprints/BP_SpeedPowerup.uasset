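; BP_SpeedPowerup is a respawning pickup that gives the ninja player character a speed boost.
; When BP_NinjaPlayerCharacter overlaps the collision box while the pickup is active, it calls the character's SpeedPowerup and plays a pickup sound at its location.
; It then hides itself and uses an IsActive flag to block retriggering until RespawnDelay elapses, when it reappears.
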(event `self.CollisionBox.OnComponentBeginOverlap`
  (params (OverlappedComponent :type "PrimitiveComponent Object Reference") (OtherActor :type "Actor Object Reference") (OtherComp :type "PrimitiveComponent Object Reference") (OtherBodyIndex :type Integer) (bFromSweep :type Boolean) (SweepResult :type "HitResult Structure (by ref)"))
  (bind _asbp_ninja_player_character (cast `/Game/Blueprints/BP_NinjaPlayerCharacter` OtherActor))
  (if (`self.bIsActive`)
    (set `self.bIsActive` false)
    (`/Game/Blueprints/BP_NinjaPlayerCharacter.SpeedPowerup` _asbp_ninja_player_character)
    (`GameplayStatics.PlaySoundAtLocation` "/Game/Audio/Sounds/S_Health_Cue.S_Health_Cue" (`self.K2_GetActorLocation`) (struct) 1.0 1.0 0.0 null null null)
    (`self.SetActorHiddenInGame` true)
    (`KismetSystemLibrary.Delay` (`self.RespawnDelay`))
    (`self.SetActorHiddenInGame` false)
    (set `self.bIsActive` true)))

(fn `UserConstructionScript`)
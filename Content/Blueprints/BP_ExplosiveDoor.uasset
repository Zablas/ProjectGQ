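; BP_ExplosiveDoor is a trigger-driven door actor that moves three mesh pieces when the ninja player character enters its box volume.
; BeginPlay caches each mesh's world transform as a base position.
; On overlap it activates a particle system and plays three timelines, each adding a vector track to one mesh's cached location.
; On exit it activates the particles again and reverses the timelines, returning the pieces along the same paths.
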(event `self.ReceiveBeginPlay`
  (set `self.SM1_Transform` (`SceneComponent.K2_GetComponentToWorld` (`self.StaticMesh`)))
  (set `self.SM2_Transform` (`SceneComponent.K2_GetComponentToWorld` (`self.StaticMesh1`)))
  (set `self.SM3_Transform` (`SceneComponent.K2_GetComponentToWorld` (`self.StaticMesh2`))))

(event `self.Box.OnComponentBeginOverlap`
  (params (OverlappedComponent :type "PrimitiveComponent Object Reference") (OtherActor :type "Actor Object Reference") (OtherComp :type "PrimitiveComponent Object Reference") (OtherBodyIndex :type Integer) (bFromSweep :type Boolean) (SweepResult :type "HitResult Structure (by ref)"))
  (cast `/Game/Blueprints/BP_NinjaPlayerCharacter` OtherActor)
  (`ActorComponent.Activate` (`self.ParticleSystem`) false)
  (`|ExecutionSequence`
    (:`then_0`
      (bind (_direction _lokacija) (`Timeline|Timeline_0` :!label _label)
        (:`Update`
          (`SceneComponent.K2_SetWorldLocation` (`self.StaticMesh`) (+ (.location (`self.SM1_Transform`)) _lokacija) false false))))
    (:`then_1`
      (bind (_direction_2 _lokacija_2) (`Timeline|Timeline_1` :!label _label_2)
        (:`Update`
          (`SceneComponent.K2_SetWorldLocation` (`self.StaticMesh1`) (+ (.location (`self.SM2_Transform`)) _lokacija_2) false false))))
    (:`then_2`
      (bind (_direction_3 _lokacija_3) (`Timeline|Timeline_2` :!label _label_3)
        (:`Update`
          (`SceneComponent.K2_SetWorldLocation` (`self.StaticMesh2`) (+ _lokacija_3 (.location (`self.SM3_Transform`))) false false))))))

(event `self.Box.OnComponentEndOverlap`
  (params (OverlappedComponent :type "PrimitiveComponent Object Reference") (OtherActor :type "Actor Object Reference") (OtherComp :type "PrimitiveComponent Object Reference") (OtherBodyIndex :type Integer))
  (cast `/Game/Blueprints/BP_NinjaPlayerCharacter` OtherActor)
  (`ActorComponent.Activate` (`self.ParticleSystem`) false)
  (`|ExecutionSequence`
    (:`then_0`
      (goto _label :!via `Reverse`))
    (:`then_1`
      (goto _label_2 :!via `Reverse`))
    (:`then_2`
      (goto _label_3 :!via `Reverse`))))

(fn `UserConstructionScript`)
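; Blue bullet actor that handles the aftermath of hitting a ninja player character, including kill and death scoring.
; PostHit casts the victim to the ninja character and passes it to a Mul-suffixed event, apparently a multicast, that plays the hit sound.
; On authority only, if the victim's health is depleted, it increments the victim's deaths and the owning shooter's kills through their player states.
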(event `self.ReceiveBeginPlay`)

(event `self.PostHit`
  (params (Character :type "WallWalkerCharacter Object Reference"))
  (bind _asbp_ninja_player_character (cast `/Game/Blueprints/BP_NinjaPlayerCharacter` Character))
  (`self.PostHit_Mul` _asbp_ninja_player_character))

(event `PostHit_Mul`
  (params (`Hit Character` :type "/Game/Blueprints/BP_NinjaPlayerCharacter Object Reference"))
  (`GameplayStatics.PlaySoundAtLocation` "/Game/Audio/Sounds/S_Hit_Cue.S_Hit_Cue" (`self.K2_GetActorLocation`) (struct) 1.0 1.0 0.0 null null null)
  (`/Engine/EditorBlueprintResources/ActorMacros.Switch Has Authority`
    (:`Authority`
      (if (<= (`WallWalkerCharacter.Health` `Hit Character`) 0.0)
        (bind _asbp_player_state (cast `/Game/Blueprints/BP_PlayerState` (`Pawn.PlayerState` `Hit Character`)))
        (`/Game/Blueprints/BP_PlayerState.IncreaseDeaths` _asbp_player_state)
        (bind _asbp_ninja_player_character (cast `/Game/Blueprints/BP_NinjaPlayerCharacter` (`self.GetOwner`)))
        (bind _asbp_player_state_2 (cast `/Game/Blueprints/BP_PlayerState` (`Pawn.PlayerState` _asbp_ninja_player_character)))
        (`/Game/Blueprints/BP_PlayerState.IncreaseKills` _asbp_player_state_2)))))

(fn `UserConstructionScript`)
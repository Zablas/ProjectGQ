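; BP_PlayerState is a player state that stores a player's name, kills and deaths and shows a join message in a kill feed.
; BeginPlay creates a UI_KillFeed widget for that player state and adds it to the viewport.
; SetName stores the name and calls JoinGameMessage, which adds a UI_JoinMessage with the username to the feed.
; The kill and death events only increment their counters, without posting to the feed.
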(event `self.ReceiveBeginPlay`
  (`self.ConstructKillFeed`))

(event `self.ReceiveTick`
  (params (DeltaSeconds :type "Float (single-precision)")))

(event `SetName`
  (params (Name :type Text))
  (bind _output_get (set `self.Name` Name))
  (`self.JoinGameMessage` _output_get))

(event `IncreaseKills`
  (`/Engine/EditorBlueprintResources/StandardMacros.IncrementInt` (`self.Kills`)))

(event `IncreaseDeaths`
  (`/Engine/EditorBlueprintResources/StandardMacros.IncrementInt` (`self.Deaths`)))

(event `JoinGameMessage`
  (params (Name :type Text))
  (bind _returnvalue (`|CreateWidget` "/Game/UI/KillFeed/UI_JoinMessage.UI_JoinMessage_C"))
  (`TextBlock.SetText` (`/Game/UI/KillFeed/UI_JoinMessage.Txt_Username` _returnvalue) Name)
  (`PanelWidget.AddChild` (`/Game/UI/KillFeed/UI_KillFeed.Feed` (`self.KillFeed`)) _returnvalue))

(fn `ConstructKillFeed`
  (bind _returnvalue (`|CreateWidget` "/Game/UI/KillFeed/UI_KillFeed.UI_KillFeed_C"))
  (bind _output_get (set `self.KillFeed` _returnvalue))
  (`UserWidget.AddToViewport` _output_get 0))

(fn `UserConstructionScript`)